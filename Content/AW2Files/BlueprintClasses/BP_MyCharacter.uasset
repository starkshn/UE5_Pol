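; Character Blueprint that performs low, thin obstacle vaults using results from its VaultSystem component.
; Tick polls CanVault and, behind a DoOnce, switches on FinalState to handle two vault variants.
; Each sets Flying mode, feeds start, loop and end locations into Motion Warping and plays its montage.
; Completion restores Walking, resets the vault and re-arms after a delay; debug prints remain and LowVault is empty.
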(event `self.ReceiveTick`
  (params (DeltaSeconds :type "Float (single-precision)"))
  (bind _vaultsystem (`self.VaultSystem`))
  (bind _startlocation (`VaultSystem.StartLocation` (`self.VaultSystem`)))
  (bind _startlocation_2 (`VaultSystem.StartLocation` (`self.VaultSystem`)))
  (bind _finalstate (`VaultSystem.FinalState` (`self.VaultSystem`)))
  (if (`VaultSystem.CanVault` (`self.VaultSystem`))
    (`/Engine/EditorBlueprintResources/StandardMacros.DoOnce` false :!label _label
      (:`Completed`
        (`KismetSystemLibrary.PrintString` (`KismetStringLibrary.Conv_VectorToString` (`VaultSystem.StartLocation` _vaultsystem)) true true (struct :`G` 0.66 :`B` 1.0 :`A` 1.0) 10.0)
        (`KismetSystemLibrary.PrintString` (`KismetStringLibrary.Conv_VectorToString` (`VaultSystem.LoopLocation` _vaultsystem)) true true (struct :`R` 0.236625 :`G` 1.0 :`A` 1.0) 10.0)
        (`KismetSystemLibrary.PrintString` (`KismetStringLibrary.Conv_VectorToString` (`VaultSystem.EndLocation` _vaultsystem)) true true (struct :`R` 1.0 :`B` 0.060021 :`A` 1.0) 10.0)
        (`KismetSystemLibrary.PrintString` (`|GetEnumeratorNameAsString` _finalstate) true true (struct :`R` 1.0 :`G` 0.879813 :`B` 0.350314 :`A` 1.0) 5.0)
        (switch `FinalVaultState` _finalstate
          (:`LowThin1`
            (`CapsuleComponent.SetCapsuleHalfHeight` (`self.CapsuleComp`) 88.0 true)
            ;[1 1 1] LowThin1Vault
            (`CharacterMovementComponent.SetMovementMode` (`self.CharacterMovement`) "MOVE_Flying" 0)
            (`KismetSystemLibrary.PrintString` (`KismetStringLibrary.Conv_VectorToString` _startlocation_2) true true (struct :`G` 0.66 :`B` 1.0 :`A` 1.0) 5.0)
            (`MotionWarpingComponent.AddOrUpdateWarpTargetFromLocationAndRotation` (`self.MotionWarping`) "MotionStart" _startlocation_2 (`self.K2_GetActorRotation`))
            (`MotionWarpingComponent.AddOrUpdateWarpTargetFromLocationAndRotation` (`self.MotionWarping`) "MotionLoop" (`VaultSystem.LoopLocation` (`self.VaultSystem`)) (`self.K2_GetActorRotation`))
            (`MotionWarpingComponent.AddOrUpdateWarpTargetFromLocationAndRotation` (`self.MotionWarping`) "MotionEnd" (`VaultSystem.EndLocation` (`self.VaultSystem`)) (`self.K2_GetActorRotation`))
            (`|PlayMontage` (`self.Mesh`) "/Game/AW2Files/Animation/Vault/LowVault/MT_LowThin1Vault_Montage.MT_LowThin1Vault_Montage"
              (:`OnCompleted`
                (`CharacterMovementComponent.SetMovementMode` (`self.CharacterMovement`) "MOVE_Walking" 0)
                (`CapsuleComponent.SetCapsuleHalfHeight` (`self.CapsuleComp`) 88.0 true)
                (`VaultSystem.ResetVault` (`self.VaultSystem`))
                (`TypedElementListLibrary.Reset` (struct))
                (`KismetSystemLibrary.Delay` 1.0)
                (goto _label :!via `Reset`))))
          (:`LowThin2`
            (`CapsuleComponent.SetCapsuleHalfHeight` (`self.CapsuleComp`) 88.0 true)
            (`CharacterMovementComponent.SetMovementMode` (`self.CharacterMovement`) "MOVE_Flying" 0)
            (`KismetSystemLibrary.PrintString` (`KismetStringLibrary.Conv_VectorToString` _startlocation) true true (struct :`G` 0.66 :`B` 1.0 :`A` 1.0) 5.0)
            (`MotionWarpingComponent.AddOrUpdateWarpTargetFromLocationAndRotation` (`self.MotionWarping`) "MotionStart" _startlocation (`self.K2_GetActorRotation`))
            (`MotionWarpingComponent.AddOrUpdateWarpTargetFromLocationAndRotation` (`self.MotionWarping`) "MotionLoop" (`VaultSystem.LoopLocation` (`self.VaultSystem`)) (`self.K2_GetActorRotation`))
            (`MotionWarpingComponent.AddOrUpdateWarpTargetFromLocationAndRotation` (`self.MotionWarping`) "MotionEnd" (`VaultSystem.EndLocation` (`self.VaultSystem`)) (`self.K2_GetActorRotation`))
            (`|PlayMontage` (`self.Mesh`) "/Game/AW2Files/Animation/Vault/LowVault/MT_LowThin2Vault2_Montage.MT_LowThin2Vault2_Montage"
              (:`OnCompleted`
                (`CharacterMovementComponent.SetMovementMode` (`self.CharacterMovement`) "MOVE_Walking" 0)
                (`CapsuleComponent.SetCapsuleHalfHeight` (`self.CapsuleComp`) 88.0 true)
                (`VaultSystem.ResetVault` (`self.VaultSystem`))
                (`TypedElementListLibrary.Reset` (struct))
                (`KismetSystemLibrary.Delay` 1.0)
                (goto _label :!via `Reset`)))))))))

(fn `LowVault`
  (params (VaultState :type "FinalVaultState Enum" :default "LowThin1")))

(fn `UserConstructionScript`)